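; AI controller for enemies that runs the BT_EnemyAI behavior tree when it possesses a pawn.
; Disconnected perception logic would set line-of-sight and target blackboard keys on sensing the player, otherwise starting a timer that clears them via StartEnemyTimer.
; A second disconnected fragment would update CanMoveTo from a visibility check.
; As wired, only the behavior tree launch runs.
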(event Custom|StartEnemyTimer
  (bind _blackboard (Variables|Default|GetBlackboard))
  (AI|Components|Blackboard|SetValueasBool _blackboard (Variables|Default|GetHasLineOfSight) false)
  (AI|Components|Blackboard|SetValueasObject _blackboard (Variables|Default|GetEnemyActor) 0))

(event EventBeginPlay)

(event EventTick
  (params (DeltaSeconds :type Float%20%28single-precision%29)))

(event EventPossess
  (params (PossessedPawn :type Pawn%20Object%20Reference))
  (AI|RunBehaviorTree "/Game/AI/BT_EnemyAI.BT_EnemyAI"))

(fn ConstructionScript)